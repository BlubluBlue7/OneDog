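; BP_James is a character Blueprint for melee combat, with player input and separate movement events for enemy use.
; Move, jump, run and EnemyMove handlers set state flags on ABP_James, whose ShouldMove and CanAttack flags gate movement and attacks.
; Mouse input starts a combo, then alternates combo types while the UpdateCombo window is open.
; Attack calls Hit on overlapping BP_James actors, setting their damage flags, including one for repeat hits.
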(event `self.ReceiveActorBeginOverlap`
  (params (OtherActor :type "Actor Object Reference"))
  (bind _overlapactorlist (`self.OverlapActorList`))
  (bind _asbp_james (cast `/Game/Character/James/BP_James` OtherActor))
  (`KismetArrayLibrary.Array_Insert` _overlapactorlist _asbp_james (`KismetArrayLibrary.Array_Length` _overlapactorlist)))

(event `self.ReceiveActorEndOverlap`
  (params (OtherActor :type "Actor Object Reference"))
  (bind _asbp_james (cast `/Game/Character/James/BP_James` OtherActor))
  (`KismetArrayLibrary.Array_RemoveItem` (`self.OverlapActorList`) _asbp_james))

(event `EnhancedInput|/Game/Input/IA_Mouse`
  (params (ActionValue :type Boolean) (ElapsedSeconds :type "Float (double-precision)") (TriggeredSeconds :type "Float (double-precision)") (InputAction :type "InputAction Object Reference" :default "/Game/Input/IA_Mouse.IA_Mouse"))
  (bind _animinstance (`self.AnimInstance`))
  (bind _animinstance_2 (`self.AnimInstance`))
  (bind _combotype (`/Game/Character/James/ABP_James.comboType` _animinstance))
  (:`Triggered`
    (if (`/Game/Character/James/ABP_James.CanAttack` _animinstance)
      (if (`|EnumEquality` _combotype "NewEnumerator0")
        (`/Game/Character/James/ABP_James.UpdateComboType` _animinstance "NewEnumerator1")
        (elif (`self.CanCombo`)
          (if (`|EnumEquality` _combotype "NewEnumerator1")
            (`/Game/Character/James/ABP_James.UpdateComboType` _animinstance_2 "NewEnumerator2")
            (else
              (`/Game/Character/James/ABP_James.UpdateComboType` _animinstance_2 "NewEnumerator1")))))))
  (:`Completed`
    (`self.Test`)))

(event `EnhancedInput|/Game/Input/IA_Run`
  (params (ActionValue :type Boolean) (ElapsedSeconds :type "Float (double-precision)") (TriggeredSeconds :type "Float (double-precision)") (InputAction :type "InputAction Object Reference" :default "/Game/Input/IA_Run.IA_Run"))
  (:`Triggered`
    (set `/Game/Character/James/ABP_James.isRunning` true (`self.AnimInstance`)))
  (:`Completed`
    (set `/Game/Character/James/ABP_James.isRunning` false (`self.AnimInstance`))))

(event `self.ReceiveBeginPlay`
  (bind _asabp_james (cast `/Game/Character/James/ABP_James` (`SkeletalMeshComponent.GetAnimInstance` (`self.Mesh`))))
  (set `self.AnimInstance` _asabp_james))

(event `self.EnemyMove`
  (bind _animinstance (`self.AnimInstance`))
  (if (`/Game/Character/James/ABP_James.shouldMove` (`self.AnimInstance`))
    (set `/Game/Character/James/ABP_James.isMoving` true _animinstance)
    (else
      (set `/Game/Character/James/ABP_James.isMoving` false _animinstance))))

(event `self.EnemyMoveEnd`
  (set `/Game/Character/James/ABP_James.isMoving` false (`self.AnimInstance`)))

(fn `Attack`
  (for _array_element (`self.OverlapActorList`)
    (bind _asbp_james (cast `/Game/Character/James/BP_James` _array_element))
    (`self.Hit` _asbp_james)))

(fn `DoJump`
  (`parent.DoJump`)
  (set `/Game/Character/James/ABP_James.isJumping` true (`self.AnimInstance`)))

(fn `DoJumpEnd`
  (`parent.DoJumpEnd`)
  (set `/Game/Character/James/ABP_James.isJumping` false (`self.AnimInstance`)))

(fn `Hit`
  (bind _animinstance (`self.AnimInstance`))
  (if (`/Game/Character/James/ABP_James.isDamaged` _animinstance)
    (set `/Game/Character/James/ABP_James.D2` true _animinstance)
    (else
      (set `/Game/Character/James/ABP_James.isDamaged` true _animinstance))))

(fn `Move`
  (params (X :type "Float (double-precision)") (Y :type "Float (double-precision)"))
  (bind _animinstance (`self.AnimInstance`))
  (if (`/Game/Character/James/ABP_James.shouldMove` (`self.AnimInstance`))
    (`parent.Move` X Y)
    (set `/Game/Character/James/ABP_James.isMoving` true _animinstance)
    (else
      (set `/Game/Character/James/ABP_James.isMoving` false _animinstance))))

(fn `MoveEnd`
  (`parent.MoveEnd`)
  (set `/Game/Character/James/ABP_James.isMoving` false (`self.AnimInstance`)))

(fn `UpdateCombo`
  (params (isEnable :type Boolean))
  (set `self.CanCombo` isEnable))

(fn `UserConstructionScript`)