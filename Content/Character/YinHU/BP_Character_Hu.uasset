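; BP_Character_Hu is the Hu character Blueprint, which links its movement handling to its animation Blueprint.
; On BeginPlay it casts the mesh's anim instance to ABP_Hu and caches it.
; Its Move and MoveEnd overrides call the parent versions, then set IsMoving on that instance to true or false.
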(event `self.ReceiveBeginPlay`
  (bind _asabp_hu (cast `/Game/Character/YinHU/ABP_Hu` (`SkeletalMeshComponent.GetAnimInstance` (`self.Mesh`))))
  (set `self.AnimInstance` _asabp_hu))

(fn `Move`
  (params (X :type "Float (double-precision)") (Y :type "Float (double-precision)"))
  (`parent.Move` X Y)
  (set `/Game/Character/YinHU/ABP_Hu.isMoving` true (`self.AnimInstance`)))

(fn `MoveEnd`
  (`parent.MoveEnd`)
  (set `/Game/Character/YinHU/ABP_Hu.isMoving` false (`self.AnimInstance`)))

(fn `UserConstructionScript`)